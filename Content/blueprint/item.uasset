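; A physics-driven shop item that a pawn grabs and drops into a cart, and that can ride through checkout.
; While grabbed, Tick steers its velocity toward the pawn's ItemTarget; arriving slows it and impulses it downward, while a timeout simply releases it.
; Checkout mode overrides this with a constant sideways velocity.
; RemoveItem later attaches it to the cart, sinks it via timeline and destroys it; OnGet spawns a dollar-sign effect.
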(event `RemoveItem`
  (params (cart :type "Actor Object Reference"))
  (`KismetSystemLibrary.Delay` 5.0)
  (`PrimitiveComponent.SetSimulatePhysics` (`self.StaticMesh`) false)
  (`self.K2_AttachToActor` cart "None" "KeepWorld" "KeepWorld" "KeepWorld" false)
  (`Timeline|Timeline`
    (:`Update`
      (`self.K2_AddActorWorldOffset` (0.0 0.0 -1.0)))
    (:`Finished`
      (`self.K2_DestroyActor`))))

(event `self.ReceiveTick`
  (params (DeltaSeconds :type "Float (single-precision)"))
  (bind _returnvalue (`self.K2_GetActorLocation`))
  (bind _returnvalue_2 (`SceneComponent.K2_GetComponentLocation` (`/Game/blueprint/cart.ItemTarget` (`self.Pawn`))))
  (if (`self.checkout mode`)
    (`PrimitiveComponent.SetPhysicsLinearVelocity` (`self.StaticMesh`) (-50.0 0.0 0.0) false "None")
    (elif (`self.beingGrabbed`)
      (`PrimitiveComponent.SetPhysicsLinearVelocity` (`self.StaticMesh`) (* (`KismetMathLibrary.GetDirectionUnitVector` _returnvalue _returnvalue_2) (`self.speed`)) false "None")
      (if (< (`KismetMathLibrary.Vector_Distance` _returnvalue _returnvalue_2) 20.0)
        (`self.endGrab` true)))))

(event `/Game/blueprint/grabbable.OnGrab`
  (params (pawn :type "/Game/blueprint/cart Object Reference"))
  (set `self.beingGrabbed` true)
  (set `self.Pawn` pawn)
  (`KismetSystemLibrary.Delay` 1.0)
  (if (`self.beingGrabbed`)
    (`self.endGrab` false)))

(event `endGrab`
  (params (`lauch into cart` :type Boolean))
  (bind _staticmesh (`self.StaticMesh`))
  (set `self.beingGrabbed` false)
  (`/Game/blueprint/cart.endGrab` (`self.Pawn`))
  (if `lauch into cart`
    (bind _returnvalue (`PrimitiveComponent.GetPhysicsLinearVelocity` _staticmesh "None"))
    (`PrimitiveComponent.SetPhysicsLinearVelocity` _staticmesh (/ _returnvalue 3.0) false "None")
    (`PrimitiveComponent.AddImpulse` _staticmesh (0.0 0.0 -300.0) "None" true)))

(event `CheckoutMode`
  (set `self.checkout mode` true))

(fn `OnGet`
  (params (cart :type "/Game/blueprint/cart Object Reference"))
  (`NiagaraFunctionLibrary.SpawnSystemAtLocation` "/Game/VFX/VFX_DollaSign.VFX_DollaSign" (`self.K2_GetActorLocation`)))

(fn `UserConstructionScript`)