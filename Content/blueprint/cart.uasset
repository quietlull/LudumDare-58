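; Player cart pawn for an on-rails item-grabbing game that rides the Track spline and triggers the Ending at its end.
; Clicked grabs trace through the cursor to send a sticky, stretching hand to grabbable actors, with the arm redrawn each tick.
; Trigger overlaps collect items into money, game-instance tallies and the HUD, or remove them.
; The camera sways with the mouse and can temporarily track targets until a set track distance.
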(event `AddEffect`
  (params (Material :type "Material Object Reference") (Duration :type "Float (double-precision)"))
  (bind _postprocesssettings (`CameraComponent.PostProcessSettings` (`self.Camera`)))
  (setmembers `PostProcessSettings` :`StructRef` _postprocesssettings :`WeightedBlendables` (make `WeightedBlendables` (`|MakeArray` (make `WeightedBlendable` 1.0 Material))))
  (`KismetSystemLibrary.Delay` Duration)
  (setmembers `PostProcessSettings` :`StructRef` _postprocesssettings :`WeightedBlendables` (make `WeightedBlendables` (`|MakeArray` (struct) :!type "WeightedBlendable Structure"))))

(event `InputAction|grab`
  (params (Key :type "Key Structure"))
  (bind _returnvalue (`SceneComponent.K2_GetComponentLocation` (`self.Camera`)))
  (:`Pressed`
    (if (not (`self.grabbing`))
      (bind _outhit (`KismetSystemLibrary.LineTraceSingle` :`Start` _returnvalue :`End` (+ _returnvalue (* (`.WorldDirection` (`PlayerController.DeprojectMousePositionToWorld` (`GameplayStatics.GetPlayerController` 0))) 1000.0)) :`TraceChannel` "TraceTypeQuery1" :`DrawTime` 1.0))
      (set `self.handmoving` true)
      (bind (_bblockinghit _binitialoverlap _time _distance _location _impactpoint _normal _impactnormal _physmat _hitactor) (`GameplayStatics.BreakHitResult` _outhit))
      (`SceneComponent.K2_SetWorldRotation` (`self.hand`) (`KismetMathLibrary.FindLookAtRotation` (`SceneComponent.K2_GetComponentLocation` (`self.handStart`)) _location) false false)
      (set `/Game/models/hand_Skeleton_AnimBlueprint.grab` false (`self.As Hand Skeleton Anim Blueprint`))
      (set `self.handtarget` _location)
      (`KismetSystemLibrary.Delay` 0.2)
      (bind _asgrabbable (cast `/Game/blueprint/grabbable` _hitactor)
        (:`then`
          (`/Game/blueprint/grabbable.OnGrab` _asgrabbable self)
          (set `self.grabbing` true)
          (set `self.handmoving` false)
          (set `/Game/models/hand_Skeleton_AnimBlueprint.grab` true (`self.As Hand Skeleton Anim Blueprint`))
          (bind _output_get (set `self.grabbedObject` _hitactor))
          (bind _returnvalue_location (`KismetMathLibrary.BreakTransform` (`KismetMathLibrary.MakeRelativeTransform` (`KismetMathLibrary.MakeTransform` _location) (`self.GetTransform` _output_get))))
          (set `self.handGrabOffset` _returnvalue_location)
          (`GameplayStatics.PlaySound2D` "/Game/Audio/StickySlap.StickySlap" 1.0 1.0 0.0 null null)
          (`KismetSystemLibrary.Delay` 0.2)
          (`GameplayStatics.PlaySound2D` "/Game/Audio/Stretch.Stretch" 1.0 1.0 0.0 null null))
        (:`CastFailed`
          (set `self.handmoving` false))))))

(event `endGrab`
  (set `self.grabbing` false))

(event `self.removeTrigger.OnComponentBeginOverlap`
  (params (OverlappedComponent :type "PrimitiveComponent Object Reference") (OtherActor :type "Actor Object Reference") (OtherComp :type "PrimitiveComponent Object Reference") (OtherBodyIndex :type Integer) (bFromSweep :type Boolean) (SweepResult :type "HitResult Structure (by ref)"))
  (bind _asitem (cast `/Game/blueprint/item` OtherActor))
  (`/Engine/EditorBlueprintResources/StandardMacros.IsValid` _asitem
    (:`Is Valid`
      (`/Game/blueprint/item.RemoveItem` _asitem self))))

(event `SetCameraTrackTarget`
  (params (TrackTarget :type "Actor Object Reference") (Distance :type "Float (double-precision)") (Continuous :type Boolean))
  (set `self.cameratarget` TrackTarget)
  (set `self.stoptrackingpos` (+ Distance (`self.position`)))
  (set `self.cameratracking` true)
  (if Continuous
    (set `self.cameracontinuous` true)
    (else
      (set `self.targetrotation` (`KismetMathLibrary.FindLookAtRotation` (`SceneComponent.K2_GetComponentLocation` (`self.camParent`)) (`self.K2_GetActorLocation` (`self.cameratarget`)))))))

(event `self.obtainItemTrigger.OnComponentBeginOverlap`
  (params (OverlappedComponent :type "PrimitiveComponent Object Reference") (OtherActor :type "Actor Object Reference") (OtherComp :type "PrimitiveComponent Object Reference") (OtherBodyIndex :type Integer) (bFromSweep :type Boolean) (SweepResult :type "HitResult Structure (by ref)"))
  (bind _ass (`self.Ass`))
  (bind _itemrecipet (`/Game/blueprint/s.itemrecipet` _ass))
  (bind _asitem (cast `/Game/blueprint/item` OtherActor))
  (if (not (`/Game/blueprint/item.obtained` _asitem))
    (set `/Game/blueprint/item.obtained` true _asitem)
    (`/Game/blueprint/item.OnGet` _asitem self)
    (bind _returnvalue (`GameplayStatics.GetObjectClass` _asitem))
    (`KismetArrayLibrary.Array_Add` (`self.items`) _returnvalue)
    (bind (_beinggrabbed _pawn _speed _value) (defaults `Object` _returnvalue))
    (bind _output_get (set `self.money` (+ (`self.money`) _value)))
    (`/Game/blueprint/ui/hudwidget.GiveMoney` (`self.hudw`) _output_get _value)
    (`GameplayStatics.PlaySound2D` "/Game/Audio/Cash_Register__Kashing___-_Sound_Effect_-_Bartholomew_Demitri_Demarcus_James_the_3rd__youtube_.Cash_Register__Kashing___-_Sound_Effect_-_Bartholomew_Demitri_Demarcus_James_the_3rd__youtube_" 1.0 1.0 0.0 null null)
    (`/Engine/EditorBlueprintResources/StandardMacros.IncrementInt` (`/Game/blueprint/s.itemnyum` _ass)
      (:`  `
        (bind (_value_2 _returnvalue_2) (`BlueprintMapLibrary.Map_Find` _itemrecipet _returnvalue))
        (if _returnvalue_2
          (`BlueprintMapLibrary.Map_Add` _itemrecipet _returnvalue (+ _value_2 1))
          (else
            (`BlueprintMapLibrary.Map_Add` _itemrecipet _returnvalue 1)))))))

(event `self.ReceiveBeginPlay`
  (bind _returnvalue (`GameplayStatics.GetPlayerController` 0))
  (`|ExecutionSequence`
    (:`then_0`
      (bind _returnvalue_2 (`GameplayStatics.GetActorOfClass` "/Game/blueprint/track.track_C"))
      (set `self.track` _returnvalue_2)
      (`WidgetBlueprintLibrary.SetInputMode_GameAndUIEx` _returnvalue null "DoNotLock" false)
      (set `PlayerController.bShowMouseCursor` true _returnvalue)
      (bind _returnvalue_3 (`|CreateWidget` "/Game/blueprint/ui/hudwidget.hudwidget_C" (`GameplayStatics.GetPlayerController` 0)))
      (`UserWidget.AddToViewport` _returnvalue_3 0)
      (set `self.hudw` _returnvalue_3)
      (bind _ashand_skeleton_anim_blueprint (cast `/Game/models/hand_Skeleton_AnimBlueprint` (`SkeletalMeshComponent.GetAnimInstance` (`self.hand`))))
      (set `self.As Hand Skeleton Anim Blueprint` _ashand_skeleton_anim_blueprint))
    (:`then_1`
      (bind _ass (cast `/Game/blueprint/s` (`GameplayStatics.GetGameInstance`)))
      (set `self.Ass` _ass))))

(event `InputAxis|look_h`
  (params (AxisValue :type "Float (single-precision)"))
  (`self.AddControllerYawInput` AxisValue))

(event `Key|LeftShift`
  (params (Key :type "Key Structure"))
  (:`Pressed`
    (set `self.speed` (+ (`self.speed`) 1000.0))))

(event `InputAxis|look_v`
  (params (AxisValue :type "Float (single-precision)"))
  (`self.AddControllerPitchInput` AxisValue))

(event `Key|Escape`
  (params (Key :type "Key Structure"))
  (:`Pressed`
    (bind _returnvalue (`|CreateWidget` "/Game/blueprint/ui/pause.pause_C"))
    (`UserWidget.AddToViewport` _returnvalue 0)
    (`GameplayStatics.SetGamePaused` true)))

(event `self.ReceiveTick`
  (params (DeltaSeconds :type "Float (single-precision)"))
  (bind _returnvalue (`WidgetLayoutLibrary.GetViewportSize`))
  (bind _camparent (`self.camParent`))
  (bind _hand (`self.hand`))
  (bind _grabbedobject (`self.grabbedObject`))
  (bind _arm (`self.arm`))
  (bind _camera (`self.Camera`))
  (bind _returnvalue_2 (`SceneComponent.K2_GetComponentToWorld` _arm))
  (bind _spline (`/Game/blueprint/track.Spline` (`self.track`)))
  (bind _returnvalue_location (`KismetMathLibrary.BreakTransform` (`KismetMathLibrary.ComposeTransforms` (`self.GetTransform` _grabbedobject) (`KismetMathLibrary.MakeTransform` (`self.handGrabOffset`)))))
  (bind _returnvalue_3 (`KismetMathLibrary.VInterpTo` (`SceneComponent.K2_GetComponentLocation` (`self.hand`)) (`KismetMathLibrary.SelectVector` (`self.handtarget`) (`SceneComponent.K2_GetComponentLocation` (`self.handStart`)) (`self.handmoving`)) DeltaSeconds 20.0))
  (`|ExecutionSequence`
    (:`then_0`
      (if (`self.moving`)
        ;[1 1 1] movement
        (bind _output_get (set `self.position` (+ (* DeltaSeconds (`self.speed`)) (`self.position`))))
        (if (> _output_get (`SplineComponent.GetSplineLength` _spline))
          (set `self.moving` false)
          (bind _returnvalue_4 (`GameplayStatics.GetActorOfClass` "/Game/blueprint/ending.ending_C"))
          (`/Game/blueprint/ending.Ending` _returnvalue_4)
          (`Widget.RemoveFromParent` (`self.hudw`))
          (bind _ass (cast `/Game/blueprint/s` (`GameplayStatics.GetGameInstance`)))
          (set `/Game/blueprint/s.money` (`self.money`) _ass)
          (else
            (`self.K2_SetActorLocation` (`SplineComponent.GetLocationAtDistanceAlongSpline` _spline _output_get "World"))
            (`self.K2_SetActorRotation` (`KismetMathLibrary.Conv_VectorToRotator` (`SplineComponent.GetTangentAtDistanceAlongSpline` _spline _output_get "World")))))))
    (:`then_1`
      ;[1 1 1] subtle camera movement
      (bind _returnvalue_5 (`WidgetLayoutLibrary.GetMousePositionOnViewport`))
      (bind (_x _y) (`KismetMathLibrary.BreakVector2D` (/ (+ _returnvalue_5 (* (/ _returnvalue 2.0) -1.0)) _returnvalue)))
      (bind _returnvalue_6 (* _y -1.0))
      (`SceneComponent.K2_SetRelativeLocation` _camera (`KismetMathLibrary.VInterpTo` (`SceneComponent.RelativeLocation` _camera) (* (`KismetMathLibrary.MakeVector` 0.0 _x _returnvalue_6) 1.0) DeltaSeconds 2.0) false false)
      (`SceneComponent.K2_SetRelativeRotation` (`self.Camera`) (`KismetMathLibrary.RInterpTo` (`SceneComponent.RelativeRotation` _camera) (* (`KismetMathLibrary.MakeRotator` 0.0 _returnvalue_6 _x) 29.0) DeltaSeconds 2.0) false false))
    (:`then_2`
      ;[1 1 1] camera track
      (if (`self.cameratracking`)
        (`|ExecutionSequence`
          (:`then_0`
            (`SceneComponent.K2_SetWorldRotation` (`self.camParent`) (`KismetMathLibrary.RInterpTo` (`SceneComponent.K2_GetComponentRotation` (`self.camParent`)) (`self.targetrotation`) DeltaSeconds 2.0) false false))
          (:`then_1`
            (if (and (`self.cameracontinuous`) (not (`self.camerareturning`)))
              (set `self.targetrotation` (`KismetMathLibrary.FindLookAtRotation` (`SceneComponent.K2_GetComponentLocation` (`self.camParent`)) (`self.K2_GetActorLocation` (`self.cameratarget`))))))
          (:`then_2`
            (if (>= (`self.position`) (`self.stoptrackingpos`))
              (set `self.camerareturning` true)
              (set `self.cameratracking` false))))
        (elif (`self.camerareturning`)
          (`SceneComponent.K2_SetRelativeRotation` _camparent (`KismetMathLibrary.RInterpTo` (`SceneComponent.RelativeRotation` _camparent) (struct) DeltaSeconds 2.0) false false)
          (if (== (`SceneComponent.RelativeRotation` (`self.camParent`)) (struct) :`ErrorTolerance` 0.01)
            (set `self.camerareturning` false)
            (set `self.cameracontinuous` false)))))
    (:`then_3`
      (`|ExecutionSequence`
        (:`then_0`
          (`/Engine/EditorBlueprintResources/StandardMacros.IsValid` _grabbedobject
            (:`Is Valid`
              (`SceneComponent.K2_SetWorldLocation` _hand (`KismetMathLibrary.SelectVector` _returnvalue_location _returnvalue_3 (`self.grabbing`)) false false))
            (:`Is Not Valid`
              (`SceneComponent.K2_SetWorldLocation` _hand _returnvalue_3 false false))))
        (:`then_1`
          (`SplineMeshComponent.SetStartAndEnd` _arm (`KismetMathLibrary.InverseTransformLocation` _returnvalue_2 (`SceneComponent.K2_GetComponentLocation` (`self.handStart`))) (0.0 0.0 0.0) (`KismetMathLibrary.InverseTransformLocation` _returnvalue_2 (`SceneComponent.K2_GetComponentLocation` (`self.hand`))) (0.0 0.0 0.0) true))))))

(fn `UserConstructionScript`)