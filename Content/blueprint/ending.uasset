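; End-of-game checkout sequence that blends the player's view to this actor and tallies the money value of the cart's items.
; A looping timer spawns each class in the Cart's item list at a scene point and puts it in checkout mode.
; One overlap box adds item values to the counter widget; another destroys items and opens the Ending level once their count reaches the spawn index.
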(event `Ending`
  (`PlayerController.SetViewTargetWithBlend` (`GameplayStatics.GetPlayerController` 0) self 1.0 "VTBlend_Linear" 0.0 false)
  (`KismetSystemLibrary.K2_SetTimerDelegate` (delegate `s[awm`) 0.3 true true)
  (bind _returnvalue (`|CreateWidget` "/Game/blueprint/ui/endingcounter.endingcounter_C"))
  (`UserWidget.AddToViewport` _returnvalue 0)
  (set `self.ui` _returnvalue))

(event `self.ReceiveBeginPlay`
  (bind _returnvalue (`GameplayStatics.GetActorOfClass` "/Game/blueprint/cart.cart_C"))
  (set `self.cart` _returnvalue))

(event `s[awm`
  (bind _i (`self.i`))
  (bind _items (`/Game/blueprint/cart.items` (`self.cart`)))
  (if (`KismetArrayLibrary.Array_IsValidIndex` _items _i)
    (bind _returnvalue (`|SpawnActorFromClass` (`|GetArrayItem` _items _i) (`SceneComponent.K2_GetComponentToWorld` (`self.Scene`)) "AdjustIfPossibleButAlwaysSpawn" "MultiplyWithRoot" null null))
    (`/Engine/EditorBlueprintResources/StandardMacros.IsValid` _returnvalue
      (:`Is Valid`
        (`KismetSystemLibrary.DelayUntilNextTick`)
        (`/Game/blueprint/item.CheckoutMode` _returnvalue)
        (`/Engine/EditorBlueprintResources/StandardMacros.IncrementInt` (`self.i`))))))

(event `self.Box.OnComponentBeginOverlap`
  (params (OverlappedComponent :type "PrimitiveComponent Object Reference") (OtherActor :type "Actor Object Reference") (OtherComp :type "PrimitiveComponent Object Reference") (OtherBodyIndex :type Integer) (bFromSweep :type Boolean) (SweepResult :type "HitResult Structure (by ref)"))
  (bind _asitem (cast `/Game/blueprint/item` OtherActor))
  (if (`/Game/blueprint/item.obtained` _asitem)
    (bind _value (`/Game/blueprint/item.value` _asitem))
    (bind _output_get (set `self.meny` (+ _value (`self.meny`))))
    (`/Game/blueprint/ui/endingcounter.GiveMoney` (`self.ui`) _output_get _value)
    (set `/Game/blueprint/item.obtained` true _asitem)))

(event `self.Box1.OnComponentBeginOverlap`
  (params (OverlappedComponent :type "PrimitiveComponent Object Reference") (OtherActor :type "Actor Object Reference") (OtherComp :type "PrimitiveComponent Object Reference") (OtherBodyIndex :type Integer) (bFromSweep :type Boolean) (SweepResult :type "HitResult Structure (by ref)"))
  (bind _asitem (cast `/Game/blueprint/item` OtherActor))
  (`self.K2_DestroyActor` _asitem)
  (bind _result (`/Engine/EditorBlueprintResources/StandardMacros.IncrementInt` (`self.2`))
    (:`  `
      (if (>= _result (`self.i`))
        (`GameplayStatics.OpenLevelBySoftObjectPtr` "/Game/Level/ending.ending")))))

(fn `UserConstructionScript`)