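; Spline track actor that drives a Cart's speed changes and camera look targets by distance along the track.
; At BeginPlay it finds the Cart, then each Tick compares its position to the next speed and camera triggers, applying one when reached.
; FindNextTrigger rescans both arrays for the nearest entries ahead.
; Outside distribution builds, the construction script marks triggers with billboards and dots each camera span along the spline.
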(event `self.ReceiveBeginPlay`
  (bind _returnvalue (`GameplayStatics.GetActorOfClass` "/Game/blueprint/cart.cart_C"))
  (set `self.cart` _returnvalue)
  (`self.FindNextTrigger` 0.0))

(event `self.ReceiveTick`
  (params (DeltaSeconds :type "Float (single-precision)"))
  (bind _cart (`self.cart`))
  (bind (_distance _speed) (break `/Game/blueprint/TrackSpeedChanger` (`self.NextSpeedChanger`)))
  (bind (_startdistance _enddistance _looktarget _continuoustrack) (break `/Game/blueprint/TrackCameraChanger` (`self.NextCameraTarget`)))
  (bind _position (`/Game/blueprint/cart.position` (`self.cart`)))
  (bind _position_2 (`/Game/blueprint/cart.position` _cart))
  (if (>= _position _distance)
    (set `/Game/blueprint/cart.speed` _speed _cart)
    (`self.FindNextTrigger` _position_2)
    (elif (>= _position _startdistance)
      (`/Game/blueprint/cart.SetCameraTrackTarget` (`self.cart`) _looktarget _enddistance _continuoustrack)
      (`self.FindNextTrigger` _position_2))))

(fn `FindNextTrigger`
  (params (Position :type "Float (double-precision)"))
  (locals (nexts :type "/Game/blueprint/TrackSpeedChanger Structure" :default (struct :`Distance` 1e+41)) (nextc :type "/Game/blueprint/TrackCameraChanger Structure" :default (struct :`StartDistance` 1e+41)))
  (bind _nextc_startdistance (break `/Game/blueprint/TrackCameraChanger` (`local.nextc`)))
  (bind _nexts_distance (break `/Game/blueprint/TrackSpeedChanger` (`local.nexts`)))
  (for _array_element (`self.SpeedChangers`)
    (bind _distance (break `/Game/blueprint/TrackSpeedChanger` _array_element))
    (if (and (< _distance _nexts_distance) (> _distance Position))
      (set `local.nexts` _array_element)))
  (for _array_element_2 (`self.CameraChangers`)
    (bind _startdistance (break `/Game/blueprint/TrackCameraChanger` _array_element_2))
    (if (and (< _startdistance _nextc_startdistance) (> _startdistance Position))
      (set `local.nextc` _array_element_2)))
  (set `self.NextSpeedChanger` (`local.nexts`))
  (set `self.NextCameraTarget` (`local.nextc`)))

(fn `MakeDottedLine`
  (params (Start :type "Float (double-precision)") (Length :type "Float (double-precision)") (Spacing :type "Float (double-precision)"))
  (locals (dist :type "Float (double-precision)"))
  (bind _returnvalue (+ (`local.dist`) (`KismetMathLibrary.FMax` Spacing 1.0)))
  (set `local.dist` _returnvalue)
  (while (< (`local.dist`) Length)
    (`AddComponent|NODE_AddBillboardComponent-3` :`RelativeTransform` (`KismetMathLibrary.MakeTransform` (+ (`SplineComponent.GetLocationAtDistanceAlongSpline` (`self.Spline`) (+ Start (`local.dist`)) "Local") (0.0 0.0 20.0))))
    (set `local.dist` _returnvalue)))

(fn `UserConstructionScript`
  (bind _spline (`self.Spline`))
  (if (not (`KismetSystemLibrary.IsPackagedForDistribution`))
    (for _array_element (`self.SpeedChangers`)
      (`AddComponent|NODE_AddBillboardComponent-0` :`RelativeTransform` (`KismetMathLibrary.MakeTransform` (`SplineComponent.GetLocationAtDistanceAlongSpline` (`self.Spline`) (`.Distance_2_06F85B884DA82F501DF141A3C4E19967` (break `/Game/blueprint/TrackSpeedChanger` _array_element)) "Local"))))
    (for _array_element_2 (`self.CameraChangers`)
      (bind (_startdistance _enddistance) (break `/Game/blueprint/TrackCameraChanger` _array_element_2))
      (`AddComponent|NODE_AddBillboardComponent-1` :`RelativeTransform` (`KismetMathLibrary.MakeTransform` (+ (`SplineComponent.GetLocationAtDistanceAlongSpline` _spline _startdistance "Local") (0.0 0.0 20.0)) (struct) (0.5 0.5 0.5)))
      (`self.MakeDottedLine` _startdistance _enddistance 50.0)
      (`AddComponent|NODE_AddBillboardComponent-2` :`RelativeTransform` (`KismetMathLibrary.MakeTransform` (+ (`SplineComponent.GetLocationAtDistanceAlongSpline` _spline (+ _enddistance _startdistance) "Local") (0.0 0.0 20.0)) (struct) (2.0 2.0 2.0))))))