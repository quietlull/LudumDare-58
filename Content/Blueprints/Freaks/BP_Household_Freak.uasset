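; Household Freak enemy that can jumpscare the player and refuses to be grabbed, immediately ending any grab.
; Its jumpscare event pauses following, swaps to a creepy face, snaps onto the cart's jumpscare target, and plays a sound with a post-process effect.
; After a short delay it detaches and restores its face and follow state; a DoOnce blocks re-triggering until then.
; BeginPlay and Tick only defer to the parent.
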(event `self.ReceiveBeginPlay`
  (`parent.ReceiveBeginPlay`))

(event `jumpscare`
  (`/Engine/EditorBlueprintResources/StandardMacros.DoOnce` false :!label _label
    (:`Completed`
      (`|ExecutionSequence`
        (:`then_0`
          (set `self.sdsadasdsad` (`self.FollowPlayer`))
          (set `self.FollowPlayer` false))
        (:`then_1`
          (`PrimitiveComponent.SetMaterial` (`self.FrontFace`) 0 "/Game/Freaks/Household_Freak_Creepy_Mat.Household_Freak_Creepy_Mat")
          (`self.K2_AttachToComponent` (`/Game/blueprint/cart.jumpscareTarget` (`self.As Cart`)) "None" "SnapToTarget" "SnapToTarget" "SnapToTarget" false)
          (`GameplayStatics.PlaySound2D` "/Engine/EditorSounds/Notifications/CompileFailed.CompileFailed" 1.0 1.0 0.0 null null)
          (`/Game/blueprint/cart.AddEffect` (`self.As Cart`) "/Game/materials/PostProcess/jumpscare_postprocess.jumpscare_postprocess" 4.0)
          (`KismetSystemLibrary.Delay` 1.0)
          (`self.K2_DetachFromActor` "KeepWorld" "KeepWorld" "KeepWorld")
          (`PrimitiveComponent.SetMaterial` (`self.FrontFace`) 0 "/Game/Freaks/Household_Freak_Mat.Household_Freak_Mat")
          (set `self.FollowPlayer` (`self.sdsadasdsad`))
          (goto _label :!via `Reset`))))))

(event `self.ReceiveTick`
  (params (DeltaSeconds :type "Float (single-precision)"))
  (`parent.ReceiveTick` DeltaSeconds))

(event `/Game/blueprint/grabbable.OnGrab`
  (params (pawn :type "/Game/blueprint/cart Object Reference"))
  (`KismetSystemLibrary.PrintString` "hey!!!!!")
  (`/Game/blueprint/cart.endGrab` pawn))

(fn `UserConstructionScript`)