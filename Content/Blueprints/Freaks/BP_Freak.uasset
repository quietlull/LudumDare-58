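; BP_Freak is a "freak" actor that can ride just ahead of the player's cart on its track, turned back toward it.
; BeginPlay caches the player pawn as a cart.
; While FollowPlayer is set, Tick interpolates the actor toward a raised, rotated point on the track spline ahead of the cart's position.
; A separate MoveToTarget event uses a timeline to lerp the actor to a given transform.
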(event `MoveToTarget`
  (params (NewPosition :type "Transform Structure"))
  (set `self.oldt` (`self.GetTransform`))
  (bind (_direction _newtrack_0) (`Timeline|Timeline`)
    (:`Update`
      (`self.K2_SetActorTransform` (`KismetMathLibrary.TLerp` (`self.oldt`) NewPosition _newtrack_0)))))

(event `self.ReceiveBeginPlay`
  (bind _ascart (cast `/Game/blueprint/cart` (`GameplayStatics.GetPlayerPawn` 0)))
  (set `self.As Cart` _ascart))

(event `self.ReceiveTick`
  (params (DeltaSeconds :type "Float (single-precision)"))
  (bind _as_cart (`self.As Cart`))
  (bind (_returnvalue_location _returnvalue_rotation) (`KismetMathLibrary.BreakTransform` (`SplineComponent.GetTransformAtDistanceAlongSpline` (`/Game/blueprint/track.Spline` (`/Game/blueprint/cart.track` _as_cart)) (+ (`/Game/blueprint/cart.position` _as_cart) 300.0) "World" false)))
  (if (`self.FollowPlayer`)
    (`/Engine/EditorBlueprintResources/StandardMacros.IsValid` _as_cart
      (:`Is Valid`
        (`self.K2_SetActorTransform` (`KismetMathLibrary.TInterpTo` (`self.GetTransform`) (`KismetMathLibrary.MakeTransform` (+ _returnvalue_location (0.0 0.0 130.0)) (`KismetMathLibrary.ComposeRotators` _returnvalue_rotation (struct :`Yaw` 180.0))) DeltaSeconds 10.0))))))

(fn `UserConstructionScript`)